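; BP_PickupItem is a configurable pickup item actor with a mesh, point light and Niagara effect.
; The construction script applies the chosen model and material, and one light color drives both the point light and the Niagara Color01 parameter.
; Its PickUp event plays a coin sound in 2D and destroys the actor.
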(event `/Game/Utils/BattleWizardPolyart/BP/BPI_Mage.Pick Up`
  (`GameplayStatics.PlaySound2D` "/Game/Utils/Interface_And_Item_Sounds/WAV/Coins_12.Coins_12" 1.0 1.0 0.0 null null)
  (`self.K2_DestroyActor`))

(fn `UserConstructionScript`
  (bind _item (`self.Item`))
  (bind _itemlight (`self.ItemLight`))
  ;[0.3 1 0.3] Set Mesh and Material
  (`StaticMeshComponent.SetStaticMesh` _item (`self.ItemModel`))
  (`PrimitiveComponent.SetMaterial` _item 0 (`self.ItemMaterial`))
  (`LightComponent.SetLightColor` (`self.PointLight`) _itemlight true)
  (`NiagaraComponent.SetVariableLinearColor` (`self.Niagara`) "Color01" _itemlight))