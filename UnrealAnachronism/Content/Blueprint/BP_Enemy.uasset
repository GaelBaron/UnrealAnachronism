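; BP_Enemy is an enemy pawn that chases the player and reacts to damage.
; On BeginPlay it uses AI MoveTo toward the player character, re-issuing the move each time it succeeds, with no handling for failure.
; AnyDamage subtracts from Health and spawns a Niagara hit effect, then enables mesh physics simulation at zero health without stopping the chase.
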(event `self.ReceiveBeginPlay`
  (`self.Chase Player`))

(event `Chase Player`
  (`|AIMoveTo` self (0.0 0.0 0.0) (`GameplayStatics.GetPlayerCharacter` 0) 120.0
    (:`OnSuccess`
      (`self.Chase Player`))))

(event `self.ReceiveAnyDamage`
  (params (Damage :type "Float (single-precision)") (DamageType :type "DamageType Object Reference") (InstigatedBy :type "Controller Object Reference") (DamageCauser :type "Actor Object Reference"))
  (set `self.Health` (- (`self.Health`) Damage))
  (`NiagaraFunctionLibrary.SpawnSystemAtLocation` "/Game/NagaraSystem/NS_Damage.NS_Damage" (`self.K2_GetActorLocation`))
  (if (<= (`self.Health`) 0.0)
    (`PrimitiveComponent.SetSimulatePhysics` (`self.Mesh`) true)))

(fn `UserConstructionScript`)